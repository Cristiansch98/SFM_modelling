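; Drivable emergency vehicle pawn with a siren, flashing lamps, an autopilot switch and two cameras.
; Enhanced Input handlers feed vehicle movement, but Tick also polls hardcoded keys and overwrites throttle, brake, steering and handbrake whenever autopilot is off.
; Polled hotkeys toggle siren, autopilot and active camera.
; The siren starts on at BeginPlay, pairing audio playback with a material Flash parameter on both lamps.
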(event `self.ReceivePossessed`
  (params (NewController :type "Controller Object Reference"))
  (`self.EnsureInputMapping`))

(event `self.OnSirenToggled`
  (params (bOn :type Boolean))
  (`self.ApplySirenLights` bOn))

(event `self.ReceiveBeginPlay`
  (`self.SetSiren` true))

(event `self.ReceiveTick`
  (params (DeltaSeconds :type "Float (single-precision)"))
  (`self.RawDriveInput`)
  (`self.RawToggles`))

(event `EnhancedInput|/Game/Input/IA_Throttle`
  (params (ActionValue :type "Float (double-precision)") (ElapsedSeconds :type "Float (double-precision)") (TriggeredSeconds :type "Float (double-precision)") (InputAction :type "InputAction Object Reference" :default "/Game/Input/IA_Throttle.IA_Throttle"))
  (:`Triggered`
    (`self.ApplyThrottle` ActionValue :!label _label))
  (:`Started`
    (`self.LogInputSeen`))
  (:`Completed`
    (goto _label)))

(event `EnhancedInput|/Game/Input/IA_Steer`
  (params (ActionValue :type "Float (double-precision)") (ElapsedSeconds :type "Float (double-precision)") (TriggeredSeconds :type "Float (double-precision)") (InputAction :type "InputAction Object Reference" :default "/Game/Input/IA_Steer.IA_Steer"))
  (:`Triggered`
    (`self.ApplySteer` ActionValue :!label _label_2))
  (:`Completed`
    (goto _label_2)))

(event `EnhancedInput|/Game/Input/IA_Handbrake`
  (params (ActionValue :type Boolean) (ElapsedSeconds :type "Float (double-precision)") (TriggeredSeconds :type "Float (double-precision)") (InputAction :type "InputAction Object Reference" :default "/Game/Input/IA_Handbrake.IA_Handbrake"))
  (:`Started`
    (`self.ApplyHandbrake` true))
  (:`Completed`
    (`self.ApplyHandbrake` false)))

(fn `ApplyHandbrake`
  (params (bOn :type Boolean))
  (`ChaosVehicleMovementComponent.SetHandbrakeInput` (`self.VehicleMovementComponent`) bOn))

(fn `ApplySirenLights`
  (params (bOn :type Boolean))
  (bind _returnvalue (select `bool` bOn :`false` 0.0 :`true` 1.0))
  (`MeshComponent.SetScalarParameterValueOnMaterials` (`self.LampLeft`) "Flash" _returnvalue)
  (`MeshComponent.SetScalarParameterValueOnMaterials` (`self.LampRight`) "Flash" _returnvalue))

(fn `ApplySteer`
  (params (Value :type "Float (double-precision)"))
  (`ChaosVehicleMovementComponent.SetSteeringInput` (`self.VehicleMovementComponent`) Value))

(fn `ApplyThrottle`
  (params (Value :type "Float (double-precision)"))
  (bind _vehiclemovementcomponent (`self.VehicleMovementComponent`))
  (`ChaosVehicleMovementComponent.SetThrottleInput` _vehiclemovementcomponent (select `bool` (> Value 0.0) :`false` 0.0 :`true` Value))
  (`ChaosVehicleMovementComponent.SetBrakeInput` _vehiclemovementcomponent (select `bool` (< Value 0.0) :`false` 0.0 :`true` (- 0.0 Value))))

(fn `EnsureInputMapping`
  (bind _returnvalue (`GameplayStatics.GetPlayerController` 0))
  (`KismetSystemLibrary.PrintString` (`KismetSystemLibrary.GetDisplayName` _returnvalue) false)
  (`self.EnableInput` self _returnvalue)
  (`WidgetBlueprintLibrary.SetInputMode_GameOnly` _returnvalue)
  (`EnhancedInputSubsystemInterface.AddMappingContext` (subsystem `EnhancedInputLocalPlayerSubsystem`) "/Game/Input/IMC_Emv.IMC_Emv" 0 (struct)))

(fn `LogInputSeen`
  (`KismetSystemLibrary.PrintString` "[emv] blueprint saw a drive key" false))

(fn `RawDriveInput`
  (bind _returnvalue (`GameplayStatics.GetPlayerController` 0))
  (bind _vehiclemovementcomponent (`self.VehicleMovementComponent`))
  (if (not (`EmvAutopilotComponent.bEnabled` (`self.Autopilot`)))
    (`ChaosVehicleMovementComponent.SetThrottleInput` _vehiclemovementcomponent (select `bool` (or (`PlayerController.IsInputKeyDown` _returnvalue "W") (`PlayerController.IsInputKeyDown` _returnvalue "Up")) :`false` 0.0 :`true` 1.0))
    (`ChaosVehicleMovementComponent.SetBrakeInput` _vehiclemovementcomponent (select `bool` (or (`PlayerController.IsInputKeyDown` _returnvalue "S") (`PlayerController.IsInputKeyDown` _returnvalue "Down")) :`false` 0.0 :`true` 1.0))
    (`ChaosVehicleMovementComponent.SetSteeringInput` _vehiclemovementcomponent (- (select `bool` (or (`PlayerController.IsInputKeyDown` _returnvalue "D") (`PlayerController.IsInputKeyDown` _returnvalue "Right")) :`false` 0.0 :`true` 1.0) (select `bool` (or (`PlayerController.IsInputKeyDown` _returnvalue "A") (`PlayerController.IsInputKeyDown` _returnvalue "Left")) :`false` 0.0 :`true` 1.0)))
    (`ChaosVehicleMovementComponent.SetHandbrakeInput` _vehiclemovementcomponent (`PlayerController.IsInputKeyDown` _returnvalue "SpaceBar"))))

(fn `RawToggles`
  (bind _returnvalue (`GameplayStatics.GetPlayerController` 0))
  (bind _returnvalue_2 (not (`self.bChaseViewRaw`)))
  (bind _returnvalue_3 (`self.K2_GetComponentsByClass` self "/Script/Engine.CameraComponent"))
  (if (`PlayerController.WasInputKeyJustPressed` _returnvalue "L")
    (`self.SetSiren` (not (`self.bSirenOnRaw`))))
  (if (`PlayerController.WasInputKeyJustPressed` _returnvalue "P")
    (set `EmvAutopilotComponent.bEnabled` (not (`EmvAutopilotComponent.bEnabled` (`self.Autopilot`))) (`self.Autopilot`)))
  (if (`PlayerController.WasInputKeyJustPressed` _returnvalue "C")
    (set `self.bChaseViewRaw` _returnvalue_2)
    (`ActorComponent.SetActive` (`|GetArrayItem` _returnvalue_3) (not _returnvalue_2) false)
    (`ActorComponent.SetActive` (`|GetArrayItem` _returnvalue_3 1) _returnvalue_2 false)))

(fn `SetSiren`
  (params (bOn :type Boolean))
  (bind _returnvalue (`self.GetComponentByClass` self "/Script/Engine.AudioComponent"))
  (set `self.bSirenOnRaw` bOn)
  (if bOn
    (`AudioComponent.Play` _returnvalue 0.0)
    (else
      (`AudioComponent.Stop` _returnvalue)))
  (`self.ApplySirenLights` bOn))

(fn `UserConstructionScript`)